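; BP_SplineTest is a construction-script tool that places copies of a static mesh at regular intervals along a spline.
; The construction script divides the spline length by Distance, then adds a NewMesh component at each step, starting from the spline's start.
; Components take only their local-space location from the spline, so they do not rotate to follow the curve.
; The event graph has no active logic.
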(fn `UserConstructionScript`
  (bind _spline (`self.Spline`))
  (bind _distance (`self.Distance`))
  (for _index (range (+ (`KismetMathLibrary.FTrunc` (`KismetMathLibrary.SafeDivide` (`SplineComponent.GetSplineLength` _spline) _distance)) 1))
    (bind _returnvalue (`AddComponent|NODE_AddStaticMeshComponent-0` :`RelativeTransform` (`KismetMathLibrary.MakeTransform` (`SplineComponent.GetLocationAtDistanceAlongSpline` _spline (* _index _distance) "Local"))))
    (`StaticMeshComponent.SetStaticMesh` _returnvalue (`self.NewMesh`))))
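; BP_TestDraw is a test Blueprint for painting on a render target with the mouse.
; While either button is held, Tick traces from the cursor and passes the hit's collision UV and a color to an M_DrawTarget dynamic material, then draws it to the target.
; Left paints red, right erases with white, and C clears DrawTest to white.
; The pawn is unpossessed during strokes, then repossessed with its saved control rotation.
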(event `self.ReceiveBeginPlay`
  (bind _returnvalue (`GameplayStatics.GetPlayerController` 0))
  (`self.EnableInput` _returnvalue)
  (set `PlayerController.bShowMouseCursor` true _returnvalue)
  (bind _returnvalue_2 (`KismetMaterialLibrary.CreateDynamicMaterialInstance` "/Game/Materials/DrawMaterial/M_DrawTarget.M_DrawTarget"))
  (set `self.DMI Brush` _returnvalue_2))

(event `self.ReceiveTick`
  (params (DeltaSeconds :type "Float (single-precision)"))
  (bind _dmi_brush (`self.DMI Brush`))
  (bind (_worldlocation _worlddirection) (`PlayerController.DeprojectMousePositionToWorld` (`GameplayStatics.GetPlayerController` 0)))
  (if (`self.bDraw`)
    (bind _outhit (`KismetSystemLibrary.LineTraceSingle` :`Start` _worldlocation :`End` (+ _worldlocation (* _worlddirection 1000)) :`TraceChannel` "TraceTypeQuery1" :`bTraceComplex` true :`DrawDebugType` "ForDuration" :`DrawTime` 0.0))
    (bind (_x _y) (`KismetMathLibrary.BreakVector2D` (`GameplayStatics.FindCollisionUV` _outhit)))
    (`MaterialInstanceDynamic.SetVectorParameterValue` _dmi_brush "DrawPosition" (make `LinearColor` _x _y))
    (if (`self.Erase`)
      (`MaterialInstanceDynamic.SetVectorParameterValue` _dmi_brush "DrawColor" (struct :`R` 1.0 :`G` 1.0 :`B` 1.0 :`A` 1.0))
      (else
        (`MaterialInstanceDynamic.SetVectorParameterValue` _dmi_brush "DrawColor" (struct :`R` 1.0 :`A` 1.0))))
    (`KismetRenderingLibrary.DrawMaterialToRenderTarget` (`self.RT_Reference`) _dmi_brush)))

(event `Key|RightMouseButton`
  (params (Key :type "Key Structure"))
  (bind _returnvalue (`GameplayStatics.GetPlayerController` 0))
  (:`Pressed`
    (set `self.Erase` true)
    (set `self.bDraw` true :!label _label)
    (set `self.ControlRotation` (`Controller.GetControlRotation` _returnvalue))
    (set `self.ControlPawn` (`Controller.K2_GetPawn` _returnvalue))
    (`Controller.UnPossess` _returnvalue))
  (:`Released`
    (set `self.Erase` false)
    (set `self.bDraw` false :!label _label_2)
    (`Controller.Possess` _returnvalue (`self.ControlPawn`))
    (`Controller.SetControlRotation` _returnvalue (`self.ControlRotation`))))

(event `Key|LeftMouseButton`
  (params (Key :type "Key Structure"))
  (:`Pressed`
    (goto _label))
  (:`Released`
    (goto _label_2)))

(event `Key|C`
  (params (Key :type "Key Structure"))
  (:`Pressed`
    (`KismetRenderingLibrary.ClearRenderTarget2D` "/Game/Materials/DrawMaterial/DrawTest.DrawTest" (struct :`R` 1.0 :`G` 1.0 :`B` 1.0 :`A` 1.0))))

(fn `UserConstructionScript`)